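; BP_OverworldPoint is a clickable overworld map point that opens either the Kerstendal or Berg level, chosen by its LevelToOpen variable.
; BeginPlay enables click and mouse-over events on the player controller, and hovering swaps the mesh material between red and white.
; A click disables hover events, blends the camera to the point while playing the LS_Fade sequence, then loads the level after a short delay.
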(event OnBeginCursorOver(StaticMesh)
  (params (TouchedComponent :type Primitive%20Component%20Object%20Reference))
  (Rendering|Material|SetMaterial (Variables|Default|GetStaticMesh) 0 "/Game/Materials/M_Red.M_Red"))

(event OnEndCursorOver(StaticMesh)
  (params (TouchedComponent :type Primitive%20Component%20Object%20Reference))
  (Rendering|Material|SetMaterial (Variables|Default|GetStaticMesh) 0 "/Game/Materials/M_White.M_White"))

(event OnClicked(StaticMesh)
  (params (TouchedComponent :type Primitive%20Component%20Object%20Reference) (ButtonPressed :type Key%20Structure :default "None"))
  (Variables|/Script/Engine.PlayerController|SetbEnableMouseOverEvents (Game|GetPlayerController 0) false)
  (Game|Player|SetViewTargetwithBlend (Game|GetPlayerController 0) self 3.0 "VTBlend_Linear" 5.0 true)
  (bind _returnvalue (Sequencer|Player|CreateLevelSequencePlayer "/Game/Blueprints/LS_Fade.LS_Fade"))
  (Sequencer|Player|Play _returnvalue :!class /Script/MovieScene.MovieSceneSequencePlayer)
  (Utilities|FlowControl|Delay 1.9)
  (switch Utilities|FlowControl|Switch|SwitchonEnum_OverworldPoint (Variables|General|GetLevelToOpen)
    (:NewEnumerator0
      (Game|OpenLevel(byObjectReference) "/Game/Maps/Kerstendal.Kerstendal"))
    (:NewEnumerator1
      (Game|OpenLevel(byObjectReference) "/Game/Maps/Berg.Berg"))))

(event EventBeginPlay
  (bind _returnvalue (Game|GetPlayerController 0))
  (Variables|/Script/Engine.PlayerController|SetbEnableClickEvents _returnvalue true)
  (Variables|/Script/Engine.PlayerController|SetbEnableMouseOverEvents _returnvalue true))

(fn ConstructionScript)