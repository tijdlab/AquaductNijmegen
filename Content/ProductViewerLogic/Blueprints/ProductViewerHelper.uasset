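; ProductViewerHelper is a product viewer helper that collects the mesh actors attached beneath a given actor.
; CreateArrayObject walks the attachment hierarchy level by level, looping without recursion and queuing children that have their own attachments as next parents.
; It returns descendants that are StaticMeshActors or contain StaticMeshComponents, without testing the starting actor itself.
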(fn ConstructionScript)

(fn CreateArrayObject
  (params (ArrayElement :type Actor%20Object%20Reference%20%28by%20ref%29))
  (Utilities|Array|Add (LocalVariables|GetNewParentActorsFound) ArrayElement)
  (LocalVariables|SetCurrentParentActors (LocalVariables|GetNewParentActorsFound) :!label _label)
  (Utilities|Array|Clear (LocalVariables|GetNewParentActorsFound))
  (if (>= (Utilities|Array|Length (LocalVariables|GetCurrentParentActors)) 1)
    (for _array_element (LocalVariables|GetCurrentParentActors)
      (bind _output_get (LocalVariables|SetCurrentAttachedActors (Actor|GetAttachedActors _array_element)))
      (LocalVariables|SetCurrentAttachedActors_Lenght (- (Utilities|Array|Length _output_get) 1))
      (for _index (range 0 (LocalVariables|GetCurrentAttachedActors_Lenght))
        (if (>= (Utilities|Array|Length (Actor|GetAttachedActors (Utilities|Array|Get(acopy) (LocalVariables|GetCurrentAttachedActors) _index))) 1)
          (Utilities|Array|Add (LocalVariables|GetNewParentActorsFound) (Utilities|Array|Get(acopy) (LocalVariables|GetCurrentAttachedActors) _index)))
        (Utilities|Casting|CastToStaticMeshActor (Utilities|Array|Get(acopy) (LocalVariables|GetCurrentAttachedActors) _index)
          (:then
            (Utilities|Array|Add (LocalVariables|GetActorMeshArray) (Utilities|Array|Get(acopy) (LocalVariables|GetCurrentAttachedActors) _index)))
          (:CastFailed
            (if (>= (Utilities|Array|Length (Actor|GetComponentsByClass (Utilities|Array|Get(acopy) (LocalVariables|GetCurrentAttachedActors) _index) "/Script/Engine.StaticMeshComponent")) 1)
              (Utilities|Array|Add (LocalVariables|GetActorMeshArray) (Utilities|Array|Get(acopy) (LocalVariables|GetCurrentAttachedActors) _index)))))))
    (goto _label)
    (else
      (return (LocalVariables|GetActorMeshArray)))))