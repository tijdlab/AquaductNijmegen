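; Touch input manager for a product viewer that sets itself as the player's view target and turns single-finger drags into orbit interaction.
; Each Tick it polls touch state, compares it with the previous frame for press, release and swipe speed, then runs the parent Tick.
; On press it traces under the finger for tagged models; release sets an interest point.
; Pinch zoom and two-finger translation logic exist but are disconnected.
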(event EventBeginPlay
  (bind _returnvalue (Game|GetPlayerController 0))
  (|CallParentFunction)
  (Utilities|FlowControl|Sequence
    (:then_0
      ;[1 1 1] Setup the Camera
      (Game|Player|SetViewTargetwithBlend (Game|GetPlayerController 0) self 0.0 "VTBlend_Linear" 0.0 false))
    (:then_1
      ;[1 1 1] Setup the Input modes
      (Input|EnableInput _returnvalue)
      (Variables|/Script/Engine.PlayerController|SetbEnableTouchEvents _returnvalue true))))

(event EventTick
  (params (DeltaSeconds :type Float%20%28single-precision%29))
  (bind _returnvalue (Game|GetPlayerController 0))
  (bind (_locationx _locationy _biscurrentlypressed) (Class|PlayerController|GetInputTouchState _returnvalue "Touch1"))
  (bind (_locationx_2 _locationy_2 _biscurrentlypressed_2) (Class|PlayerController|GetInputTouchState _returnvalue "Touch2"))
  (Utilities|FlowControl|Sequence
    (:then_0
      ;[1 1 1] Get Current Touch Values
      (Variables|Default|SetTouch1Loc (Math|Vector2D|MakeVector2D _locationx _locationy))
      (Variables|Default|SetIsTouch1Pressed _biscurrentlypressed)
      (Variables|Default|SetIsTouch2Pressed _biscurrentlypressed_2)
      (Variables|Default|SetIs2TouchesPressed (and _biscurrentlypressed _biscurrentlypressed_2)))
    (:then_1
      ;[1 1 1] Detect Drag on Single Touch Input
      (if (Variables|Default|GetWasTouch1Pressed)
        (Variables|Default|SetInteractSwipeSpeed (* (* (- (Variables|Default|GetPrevTouch1Loc) (Variables|Default|GetTouch1Loc)) (Variables|Default|GetSwipeScale)) "(X=-1.000000,Y=1.000000)"))))
    (:then_2
      ;[1 1 1] Detect Start Touch
      (if (and (not (Variables|Default|GetWasTouch1Pressed)) (Variables|Default|GetIsTouch1Pressed))
        (Variables|Default|SetStartInteractingLocation (Variables|Default|GetTouch1Loc))
        (CallFunction|GetHitLocModel false)
        (Variables|Default|SetIsOrbiting true)
        (CallFunction|SetReversedRotation)))
    (:then_3
      ;[1 1 1] Detect Stop Touch
      (if (and (Variables|Default|GetWasTouch1Pressed) (not (Variables|Default|GetIsTouch1Pressed)))
        (Variables|Default|SetStopInteractingLocation (Variables|Default|GetTouch1Loc))
        (CallFunction|SetInterestPoint)
        (Variables|Default|SetIsOrbiting false)))
    (:then_4)
    (:then_5)
    (:then_6
      ;[1 1 1] Keep Touch Values for next frames
      (Variables|Default|SetPrevTouch1Loc (Variables|Default|GetTouch1Loc))
      (Variables|Default|SetWasTouch1Pressed (Variables|Default|GetIsTouch1Pressed))
      (Variables|Default|SetWas2TouchesPressed (Variables|Default|GetIs2TouchesPressed)))
    (:then_7
      (|CallParentFunction DeltaSeconds))))

(event Input|AxisEvents|InputAxisPinch
  (params (AxisValue :type Float%20%28single-precision%29))
  ;[1 1 1] ZOOM
)

(fn ConstructionScript)

(fn GetHitLocModel
  (params (ExcludeModels :type Boolean))
  (bind _returnvalue (Game|GetPlayerController 0))
  (bind _array (Utilities|Array|MakeArray "ObjectTypeQuery2" "ObjectTypeQuery1"))
  (bind (_hitresult _returnvalue_2) (Class|PlayerController|GetHitResultUnderFingerforObjects _returnvalue "Touch1" _array true))
  (bind (_bblockinghit _binitialoverlap _time _distance _location _impactpoint _normal _impactnormal _physmat _hitactor) (Collision|BreakHitResult _hitresult))
  (if _returnvalue_2
    (if (!= (Utilities|Array|FindItem (Variables|/Script/Engine.Actor|GetTags _hitactor) (Utilities|Array|Get(acopy) (Variables|Default|GetInteractiveTag))) -1)
      (Variables|Default|SetTraceHitLocation _location)
      (Variables|Default|SetHitModel _hitactor)))
  (return false "0, 0, 0"))